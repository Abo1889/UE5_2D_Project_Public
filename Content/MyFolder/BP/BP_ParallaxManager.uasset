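; BP_ParallaxManager is an actor that creates parallax scrolling across three background layers (far, mid and near) as the camera moves along X.
; On BeginPlay it caches the player character's camera component, the camera's starting X and each layer's starting relative X.
; Each Tick it offsets every layer's X by the camera's displacement times a per-layer factor, keeping fixed Y depths and each layer's current Z.
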(event EventBeginPlay
  (bind _output_get (Variables|Default|SetCameraRef (Actor|GetComponentbyClass (Game|GetPlayerCharacter 0) "/Script/Engine.CameraComponent")))
  (Variables|Default|SetCamInitX (.X (Math|Vector|BreakVector (Transformation|GetWorldLocation _output_get))))
  (Variables|Default|SetFarInitX (.X (Math|Vector|BreakVector (Variables|/Script/Engine.SceneComponent|GetRelativeLocation (Variables|Default|GetFarBg)))))
  (Variables|Default|SetMidInitX (.X (Math|Vector|BreakVector (Variables|/Script/Engine.SceneComponent|GetRelativeLocation (Variables|Default|GetMidBg)))))
  (Variables|Default|SetNearInitX (.X (Math|Vector|BreakVector (Variables|/Script/Engine.SceneComponent|GetRelativeLocation (Variables|Default|GetNearBg))))))

(event Collision|EventActorBeginOverlap
  (params (OtherActor :type Actor%20Object%20Reference)))

(event EventTick
  (params (DeltaSeconds :type Float%20%28single-precision%29))
  (bind _cameraref (Variables|Default|GetCameraRef))
  (bind _caminitx (Variables|Default|GetCamInitX))
  (bind _returnvalue (Transformation|GetWorldLocation _cameraref))
  (bind _x (Math|Vector|BreakVector _returnvalue))
  (bind _returnvalue_2 (- _x _caminitx))
  (Transformation|SetRelativeLocation (Variables|Default|GetFarBg) (Math|Vector|MakeVector (+ (* _returnvalue_2 0.1) (Variables|Default|GetFarInitX)) 5e+02 (.Z (Math|Vector|BreakVector (Variables|/Script/Engine.SceneComponent|GetRelativeLocation (Variables|Default|GetFarBg))))) false false)
  (Transformation|SetRelativeLocation (Variables|Default|GetMidBg) (Math|Vector|MakeVector (+ (* _returnvalue_2 0.5) (Variables|Default|GetMidInitX)) 3e+02 (.Z (Math|Vector|BreakVector (Variables|/Script/Engine.SceneComponent|GetRelativeLocation (Variables|Default|GetMidBg))))) false false)
  (Transformation|SetRelativeLocation (Variables|Default|GetNearBg) (Math|Vector|MakeVector (+ (* _returnvalue_2 1.0) (Variables|Default|GetNearInitX)) 1.5e+02 (.Z (Math|Vector|BreakVector (Variables|/Script/Engine.SceneComponent|GetRelativeLocation (Variables|Default|GetNearBg))))) false false))

(fn ConstructionScript)